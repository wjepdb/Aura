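; GA_MeleeAttack is a gameplay ability for a melee attack that plays the goblin spear attack montage.
; On activation it turns the avatar toward its combat target through CombatInterface, then plays the montage and waits for the melee montage gameplay event.
; When the event arrives it draws a randomly colored debug sphere at the combat socket location and ends the ability, with no damage applied yet.
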(event `self.K2_ActivateAbility`
  (bind _returnvalue (`self.GetAvatarActorFromActorInfo`))
  (bind _returnvalue_2 (message `EnemyInterface.GetCombatTarget` _returnvalue))
  (bind _ascombat_interface (cast `CombatInterface` _returnvalue))
  (`CombatInterface.UpdateFacingTarget` _ascombat_interface (`Actor.K2_GetActorLocation` _returnvalue_2))
  (`AbilityTask_PlayMontageAndWait.CreatePlayMontageAndWaitProxy` "None" "/Game/Assets/Enemies/Goblin/Animations/Spear/AM_Attack_GoblinSpear.AM_Attack_GoblinSpear"
    (:`then`
      (`AbilityTask_WaitGameplayEvent.WaitGameplayEvent` (struct :`TagName` "Event.Montage.Attack.Melee") null
        (:`EventReceived`
          (bind _returnvalue_3 (message `CombatInterface.GetCombatSocketLocation` _returnvalue))
          (`KismetSystemLibrary.DrawDebugSphere` _returnvalue_3 10.0 12 (select `int` (`KismetMathLibrary.RandomIntegerInRange` 0 2) :`0` (`KismetMathLibrary.LinearColor_Red`) :`1` (`KismetMathLibrary.LinearColor_Green`) :`2` (`KismetMathLibrary.LinearColor_Blue`)) 3.0 1.0)
          (`self.K2_EndAbility`))))))